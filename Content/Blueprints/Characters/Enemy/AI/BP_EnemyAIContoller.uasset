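; Enemy AI controller that runs BT_EnemyTree on possession and uses AI perception to drive chasing of the player.
; A perception update for a BP_Player cancels the chase timer, sets IsChase and stores the player as PlayerActor in the Blackboard.
; An update for any other actor starts a short timer that then clears both keys.
; Sensing success is not checked, only the actor's class.
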(event `self.ReceiveBeginPlay`)

(event `self.ReceivePossess`
  (params (PossessedPawn :type "Pawn Object Reference"))
  (`self.RunBehaviorTree` "/Game/Blueprints/Characters/Enemy/AI/BT_EnemyTree.BT_EnemyTree"))

(event `self.AIPerception.OnTargetPerceptionUpdated`
  (params (Actor :type "Actor Object Reference") (Stimulus :type "AIStimulus Structure"))
  (bind _blackboard (`self.Blackboard`))
  (bind _asbp_player (cast `/Game/Blueprints/Characters/Player/BP_Player` Actor)
    (:`then`
      (`KismetSystemLibrary.K2_ClearAndInvalidateTimerHandle` (`self.ChaseTimer`))
      (`BlackboardComponent.SetValueAsBool` _blackboard (`self.IsChase`) true)
      (`BlackboardComponent.SetValueAsObject` _blackboard (`self.PlayerActor`) _asbp_player))
    (:`CastFailed`
      (bind _returnvalue (`KismetSystemLibrary.K2_SetTimerDelegate` (delegate `StopChase`) 2.0))
      (set `self.ChaseTimer` _returnvalue))))

(event `StopChase`
  (bind _blackboard (`self.Blackboard`))
  (`BlackboardComponent.SetValueAsBool` _blackboard (`self.IsChase`) false)
  (`BlackboardComponent.SetValueAsObject` _blackboard (`self.PlayerActor`) null))

(fn `UserConstructionScript`)