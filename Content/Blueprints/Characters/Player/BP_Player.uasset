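; Player character Blueprint that plays the scripted get-up and door-opening sequences.
; BeginPlay binds handlers for game start and door opening; the get-up montage switches player state and snaps the character to a fixed position at its end notify.
; Door-opening montage notifies play and reverse a timeline that swings the passed door's mesh, with its tip hidden when the timeline finishes.
; On montage completion, the character jumps forward along world X.
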(event `self.ReceiveBeginPlay`
  ;[1 1 1] BiginPlay
  (`parent.ReceiveBeginPlay`)
  (add `self.StartGame` (`|CreateDelegate` :!event `StartGameEvent`))
  (add `self.OpenDoor` (`|CreateDelegate` :!event `OpenDoorEvent`)))

(event `StartGameEvent`
  ;[1 1 1] 开始游戏时播放起床蒙太奇
  (`|PlayMontage` (`self.Mesh`) "/Game/Assets/Characters/main_man/Anim/maincharactor_getup_ani_Montage.maincharactor_getup_ani_Montage"
    (:`then`
      (set `self.CurrentPlayerState` "EPS_PlayMontage"))
    (:`OnNotifyEnd`
      (set `self.CurrentPlayerState` "EPS_Normal")
      (`self.K2_SetActorLocation` (200.0 -825.137817 112.634163)))))

(event `OpenDoorEvent` :!signature `self.OpenDoor`
  (params (Door :type "DoorInteract Object Reference"))
  (bind (_returnvalue_x _returnvalue_y _returnvalue_z) (`KismetMathLibrary.BreakVector` (`self.K2_GetActorLocation`)))
  ;[1 1 1] 开门函数广播
  (set `self.Door` Door)
  (`self.K2_SetActorRotation` (struct))
  (`|PlayMontage` (`self.Mesh`) "/Game/Assets/Characters/main_man/Anim/maincharactor_opendoor_ani_Montage.maincharactor_opendoor_ani_Montage"
    (:`OnCompleted`
      (`self.K2_SetActorLocation` (`KismetMathLibrary.MakeVector` (+ _returnvalue_x 749.0) _returnvalue_y _returnvalue_z)))
    (:`OnNotifyBegin`
      (bind (_direction _opendoor) (`Timeline|时间轴_0` :!via `PlayFromStart` :!label _label)
        (:`Update`
          (`SceneComponent.K2_SetRelativeRotation` (`Interact.MeshComp` (`self.Door`)) (`KismetMathLibrary.MakeRotator` 0.0 0.0 _opendoor) false false))
        (:`Finished`
          (`SceneComponent.SetVisibility` (`Interact.TipsComp` (`self.Door`)) false false))))
    (:`OnNotifyEnd`
      (goto _label :!via `Reverse`))))

(fn `UserConstructionScript`
  (`parent.UserConstructionScript`))