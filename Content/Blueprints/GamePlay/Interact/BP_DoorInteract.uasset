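; BP_DoorInteract is an interactable door that, on interaction, hides its tips component, spawns a moving subway background and asks the player to open it.
; The BP_SubwayBG actor spawns at a fixed offset from the door, and its start location is cached.
; A DoOnce-gated timeline moves the background along negative X by its Speed track, snapping it back to the start once it reaches the door's X for a looping scroll.
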(event `self.OnInteract`
  ;[1 1 1] 打开关闭门
  (`parent.OnInteract`)
  (`SceneComponent.SetVisibility` (`self.TipsComp`) false false)
  (`self.CreateSubwayBG`) ; 在开门时创建地铁背景
  (bind _asbp_player (cast `/Game/Blueprints/Characters/Player/BP_Player` (`GameplayStatics.GetPlayerCharacter` 0)))
  (`/Game/Blueprints/Characters/Player/BP_Player.OpenDoor` _asbp_player self))

(event `CreateSubwayBG`
  (bind (_returnvalue_location _returnvalue_rotation) (`KismetMathLibrary.BreakTransform` (`self.GetTransform`)))
  ;[1 1 1] 创建地铁背景
  (bind _returnvalue (`|SpawnActorFromClass` "/Game/Blueprints/GamePlay/BP_SubwayBG.BP_SubwayBG_C" (`KismetMathLibrary.MakeTransform` (+ _returnvalue_location (3629.699951 -797.780029 90.0)) _returnvalue_rotation) "Undefined" "OverrideRootScale" null null))
  (bind _output_get (set `self.Subway_BG_Ref` _returnvalue))
  ;;[1 1 1] 在创建时使用临时变量保存位置
  (set `self.SubwayBGLocation` (`self.K2_GetActorLocation` _output_get))
  (`self.LoopSubwayBG`))

(event `LoopSubwayBG`
  (bind _returnvalue_x (`KismetMathLibrary.BreakVector` (`self.K2_GetActorLocation`)))
  (bind _returnvalue (`self.K2_GetActorLocation` (`self.Subway_BG_Ref`)))
  ;[1 1 1] 循环Subway背景
  (`/Engine/EditorBlueprintResources/StandardMacros.DoOnce` false
    (:`Completed`
      (bind (_direction _speed) (`Timeline|SubwayBGTransform` :!via `PlayFromStart`)
        (:`Update`
          (`self.K2_SetActorLocation` (`self.Subway_BG_Ref`) (- _returnvalue (`KismetMathLibrary.MakeVector` _speed)) false false)
          (if (<= (.x _returnvalue) _returnvalue_x)
            (`self.K2_SetActorLocation` (`self.Subway_BG_Ref`) (`self.SubwayBGLocation`) false false)))))))

(fn `UserConstructionScript`)