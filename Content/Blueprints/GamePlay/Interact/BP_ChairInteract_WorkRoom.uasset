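; BP_ChairInteract_WorkRoom is an interactable Blueprint that, by its name, serves as the chair in the work room.
; On BeginPlay it casts the first player pawn to BP_Player and caches the reference.
; OnInteract runs the parent behavior, then passes itself to the player's CallChairInteract only if the player's state is Normal, leaving the chair logic to BP_Player.
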(event `self.ReceiveBeginPlay`
  (bind _asbp_player (cast `/Game/Blueprints/Characters/Player/BP_Player` (`GameplayStatics.GetPlayerPawn` 0)))
  (set `self.As BP Player` _asbp_player))

(event `self.OnInteract`
  (`parent.OnInteract`)
  (if (`|EnumEquality` (`CharacterBase.CurrentPlayerState` (`self.As BP Player`)) "EPS_Normal")
    (`/Game/Blueprints/Characters/Player/BP_Player.ChairInteract` (`self.As BP Player`) self)))

(fn `UserConstructionScript`)