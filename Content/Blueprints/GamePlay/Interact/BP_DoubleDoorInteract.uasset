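; BP_DoubleDoorInteract is an interactable double door gated behind a puzzle minigame.
; On interact it runs the parent logic, hides its tip component, and shows the WBP_SmallGame1 widget with mouse cursor and Game-and-UI input, setting the player's state to None.
; The widget's Success event tells BP_Player to open the double door, passing this actor.
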(event `self.OnInteract`
  ;[1 1 1] 互动
  (`parent.OnInteract`)
  (`SceneComponent.SetVisibility` (`self.TipsComp`) false false)
  (`self.CreateGame1`))

(event `CreateGame1`
  (bind _returnvalue (`GameplayStatics.GetPlayerController` 0))
  ;[1 1 1] 创建解密1
  (bind _returnvalue_2 (`|CreateWidget` "/Game/Blueprints/GamePlay/SmallGame/WBP_SmallGame1.WBP_SmallGame1_C"))
  (add `/Game/Blueprints/GamePlay/SmallGame/WBP_SmallGame1.Success` _returnvalue_2 (delegate `SuccessEvent`))
  (`UserWidget.AddToViewport` _returnvalue_2 0)
  (`WidgetBlueprintLibrary.SetInputMode_GameAndUIEx` _returnvalue null)
  (set `PlayerController.bShowMouseCursor` true _returnvalue)
  (bind _asbp_player (cast `/Game/Blueprints/Characters/Player/BP_Player` (`GameplayStatics.GetPlayerPawn` 0)))
  (set `CharacterBase.CurrentPlayerState` "EPS_None" _asbp_player))

(event `SuccessEvent`
  ;[1 1 1] 解密成功调用开门
  (bind _asbp_player (cast `/Game/Blueprints/Characters/Player/BP_Player` (`GameplayStatics.GetPlayerCharacter` 0)))
  (`/Game/Blueprints/Characters/Player/BP_Player.OpenDoubleDoor` _asbp_player self))

(fn `UserConstructionScript`)