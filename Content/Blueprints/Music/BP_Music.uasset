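; BP_Music is an actor that plays background audio through two media players and switches it to subway ambience on an event.
; On BeginPlay it opens the first source and binds that player's end-reached event to Openbgm, which reopens both sources as a loop.
; The Subway event swaps in subway noise and crowd chatter sources, then calls Openbgm to start both immediately.
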(event `self.ReceiveBeginPlay`
  (bind _media1 (`self.Media1`))
  (`MediaPlayer.OpenSource` _media1 (`self.Media Source1`))
  (add `MediaPlayer.OnEndReached` _media1 (delegate `Openbgm`))
  (add `self.Subway` (delegate `Subway_Event`)))

(event `Openbgm`
  (`MediaPlayer.OpenSource` (`self.Media1`) (`self.Media Source1`))
  (`MediaPlayer.OpenSource` (`self.Media2`) (`self.Media Source2`)))

(event `Subway_Event`
  (set `self.Media Source1` "/Game/Assets/Music/Subway/地铁声音_Subway_Sound__爱给网_aigei_com.地铁声音_Subway_Sound__爱给网_aigei_com")
  (set `self.Media Source2` "/Game/Assets/Music/Subway/地铁人群喋喋不休说话_爱给网_aigei_com.地铁人群喋喋不休说话_爱给网_aigei_com")
  (`self.Openbgm`))

(fn `UserConstructionScript`)